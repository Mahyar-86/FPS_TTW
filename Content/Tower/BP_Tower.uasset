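; BP_Tower is a turret that turns toward any Character its PawnSensing component sees and fires from two muzzles.
; Each sighting interpolates the actor's yaw and the Tower component's yaw and clamped pitch toward the target.
; It also restarts a one-second retriggerable delay, which spawns a BP_Bullet at both spawn points only once it elapses without another sighting.
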(event OnSeePawn(PawnSensing)
  (params (Pawn :type Pawn%20Object%20Reference))
  (bind _ascharacter (Utilities|Casting|CastToCharacter Pawn))
  (Utilities|FlowControl|Sequence
    (:then_0
      (Transformation|SetWorldRotation (Variables|Default|GetTower) (Math|Rotator|MakeRotator 0.0 (Math|Float|Clamp(Float) (.pitch (Math|Interpolation|RInterpTo (Transformation|GetActorRotation) (Math|Rotator|FindLookatRotation (Transformation|GetActorLocation) (Transformation|GetActorLocation _ascharacter)) (Utilities|Time|GetWorldDeltaSeconds) (* 2e+01 5.0))) -2e+01 2e+01) (.yaw (Math|Interpolation|RInterpTo (Transformation|GetActorRotation) (Math|Rotator|FindLookatRotation (Transformation|GetActorLocation) (Transformation|GetActorLocation _ascharacter)) (Utilities|Time|GetWorldDeltaSeconds) (* 2e+01 5.0)))) false false)
      (Transformation|SetActorRotation (Math|Rotator|MakeRotator 0.0 0.0 (.yaw (Math|Interpolation|RInterpTo (Transformation|GetActorRotation) (Math|Rotator|FindLookatRotation (Transformation|GetActorLocation) (Transformation|GetActorLocation _ascharacter)) (Utilities|Time|GetWorldDeltaSeconds) (* 2e+01 5.0))))))
    (:then_1
      (Utilities|FlowControl|RetriggerableDelay 1.0)
      (Game|SpawnActorfromClass "/Game/Tower/BP_Bullet.BP_Bullet_C" (Transformation|GetWorldTransform (Variables|Default|GetBulletSpawn1)) "Undefined" "MultiplyWithRoot" 0 0)
      (Game|SpawnActorfromClass "/Game/Tower/BP_Bullet.BP_Bullet_C" (Transformation|GetWorldTransform (Variables|Default|GetBulletSpawn2)) "Undefined" "MultiplyWithRoot" 0 0))))

(fn ConstructionScript)