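; Auto-targeting defense tower that fires bullets by default and can switch to a laser mode with beam effect.
; Each tick it picks the nearest visible pawn via sphere overlap, smoothly rotates its pitch-clamped head, and fires on cooldown when a dot product confirms aim.
; Shots spawn a projectile and sound, plus a line trace setting the Niagara beam end and impact emitter.
; Tower manager checks drive laser-only range, fire-rate and damage upgrade functions.
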(event Custom|FireBullet
  (bind _head (Variables|Default|GetHead))
  (bind _returnvalue (Transformation|GetWorldTransform _head))
  ;[0.4333 1 0.4902] FireBullet
  (Variables|Private|SetTimeOfLastFire (Utilities|Time|GetGameTimeinSeconds))
  (Utilities|FlowControl|Sequence
    (:then_0
      (goto _label Reset))
    (:then_1
      (Utilities|FlowControl|DoN 10 :!label _label
        (:Exit
          (CallFunction|SpawnLaser)
          (Game|SpawnActorfromClass "/Game/Tower/BP_Bullet.BP_Bullet_C" (Math|Transform|MakeTransform (+ (.location _returnvalue) "5.000000,0.000000,0.000000") (.rotation _returnvalue) (.scale _returnvalue)) "Undefined" "MultiplyWithRoot" 0 0)
          (Audio|SpawnSoundAttached "/Game/MilitaryWeapSilver/Sound/Pistol/Wavs/PistolA_Fire_ST06.PistolA_Fire_ST06" (Variables|Default|GetHead) "None" "0, 0, 0" "0, 0, 0" "KeepRelativeOffset" false 1.0 1.0 0.0 "/Game/Sounds/SA_SoundAttenuation.SA_SoundAttenuation" 0))))))

(event Custom|SpawnLaser
  (bind _ns_laser (Variables|Default|GetNS_Laser))
  (bind _returnvalue (Transformation|GetWorldLocation _ns_laser))
  ;[1 0.06771 0.06771] FireLaiser
  (bind (_outhit _returnvalue_2) (Collision|LineTraceByChannel _returnvalue (+ _returnvalue (* (Math|Vector|GetForwardVector _ns_laser) 5e+05)) "TraceTypeQuery1" false 0 "None"))
  (if _returnvalue_2
    _
    (else
      _))
  (CallFunction|ActiveLaser (.ImpactPoint (Collision|BreakHitResult _outhit))))

(event Custom|FireRateCheck
  (if (not (!= (Variables|/Game/Tower/BP_TowerManager.BP_TowerManager_C|GetFRTime (Variables|Default|GetTowerManager)) 1))
    (CallFunction|UpgradeFireRate 0.1)))

(event Custom|ActiveLaser
  (params (Param :type Vector))
  (bind _ns_laser (Variables|Default|GetNS_Laser))
  ;[1 0.06771 0.06771] FireLaiser
  (Components|Activation|SetActive _ns_laser true false)
  (Effects|Components|ParticleSystem|SetVectorParameter _ns_laser "Beam End" Param)
  (Effects|SpawnEmitteratLocation "/Game/Realistic_Starter_VFX_Pack_Vol2/Particles/Explosion/P_Molotov.P_Molotov" (.ImpactPoint (Collision|BreakHitResult (stale Custom|SpawnLaser _outhit))) "0, 0, 0" "0.200000,0.200000,0.200000"))

(event Custom|FireLaiser
  (bind _head (Variables|Default|GetHead))
  (bind _returnvalue (Transformation|GetWorldTransform _head))
  ;[1 0.06771 0.06771] FireLaiser
  (Variables|Private|SetTimeOfLastFire (Utilities|Time|GetGameTimeinSeconds))
  (Utilities|FlowControl|Sequence
    (:then_0
      (goto _label Reset))
    (:then_1
      (Utilities|FlowControl|DoN 10 :!label _label
        (:Exit
          (CallFunction|SpawnLaser)
          (Game|SpawnActorfromClass "/Game/Tower/BP_LaiserBulet.BP_LaiserBulet_C" (Math|Transform|MakeTransform (+ (.location _returnvalue) "5.000000,0.000000,0.000000") (.rotation _returnvalue) (.scale _returnvalue)) "Undefined" "MultiplyWithRoot" 0 0)
          (Audio|SpawnSoundAttached "/Game/Sounds/Towers/Laser.Laser" (Variables|Default|GetHead) "None" "0, 0, 0" "0, 0, 0" "KeepRelativeOffset" false 1.0 1.0 0.0 "/Game/Sounds/SA_SoundAttenuation.SA_SoundAttenuation" 0))))))

(event Custom|CheckIfTowerIsLaiser
  (bind _islaiser (Variables|TimesUpgraded|GetIsLaiser))
  (if (not _islaiser)
    (CallFunction|UpgradetoLaiser _islaiser)))

(event Custom|UpgradeToLaiser
  (params (IsLaiser :type Boolean))
  (if IsLaiser
    (Variables|TimesUpgraded|SetIsLaiser (Variables|Default|GetTrue))
    (else
      (Variables|TimesUpgraded|SetIsLaiser (Variables|Default|GetTrue)))))

(event Custom|SetDefaults
  (Variables|Upgradeble|Setsensing_range (Variables|DefaultValues|GetDefaultSensingRange))
  (Variables|Upgradeble|SetRateOfFire (Variables|DefaultValues|GetDefaultFireRate))
  (Variables|Upgradeble|SetDamage (Variables|DefaultValues|GetDefaultDamage)))

(event Custom|BulletTower
  (Variables|TimesUpgraded|SetIsLaiser (Variables|Default|GetFalse))
  (Development|SetHiddeninGame (Variables|Default|GetNS_Laser) (Variables|Default|GetTrue) false))

(event Custom|DamageCheck
  (if (not (!= (Variables|/Game/Tower/BP_TowerManager.BP_TowerManager_C|GetDTime (Variables|Default|GetTowerManager)) 1))
    (CallFunction|UpgradeBulletDamage 5.0)))

(event Custom|ChekRAnge
  (if (not (!= (Variables|/Game/Tower/BP_TowerManager.BP_TowerManager_C|GetRTime (Variables|Default|GetTowerManager)) 1))
    (CallFunction|UpgradeRange 1e+03)))

(event EventBeginPlay
  (CallFunction|SetDefaults)
  (CallFunction|BulletTower)
  (bind _returnvalue (Actor|GetActorOfClass "/Game/Tower/BP_TowerManager.BP_TowerManager_C"))
  (Variables|Default|SetTowerManager _returnvalue))

(event EventTick
  (params (DeltaSeconds :type Float%20%28single-precision%29))
  (Private|FindBestTarget)
  (Variables|Private|GetTarget
    (:then
      (Private|UpdateTowerRotation DeltaSeconds)
      (Private|UpdateFire))
    (:else)))

(fn ConstructionScript)

(fn FindBestTarget
  ;[1 1 1] set the best distance var to the max
  (LocalVariables|Setbest_distance%28local%29 (+ (Variables|Upgradeble|Getsensing_range) 1.0))
  ;[1 1 1] detect zombies entering the sence zone
  (bind _outactors (Collision|SphereOverlapActors (Transformation|GetActorLocation) (Variables|Upgradeble|Getsensing_range) (Utilities|Array|MakeArray "ObjectTypeQuery3") 0 (Utilities|Array|MakeArray (Variables|Default|GetPlayer))))
  ;[1 1 1] looping through the array to find the closest target to the tower
  (for _array_element _outactors
    (bind _output_get (LocalVariables|Setcurrent_target%28local%29 _array_element))
    (Utilities|Casting|CastToBP_FirstPersonCharacter _output_get
      (:CastFailed
        (bind _output_get_2 (LocalVariables|Setcurrent_distance%28local%29 (Transformation|GetDistanceTo _output_get self)))
        (if (or (< _output_get_2 (LocalVariables|Getbest_distance%28local%29)) (not (Utilities|IsValid (LocalVariables|Getbest_target%28local%29)))) ; is this is the closest so far?
          (bind _result (CallFunction|HasLineOfSight (Transformation|GetWorldLocation (Variables|Default|GetHead)) (Transformation|GetActorLocation (LocalVariables|Getcurrent_target%28local%29)) (Utilities|Array|MakeArray self (LocalVariables|Getcurrent_target%28local%29) 0)))
          (if _result
            (LocalVariables|Setbest_target%28local%29 (LocalVariables|Getcurrent_target%28local%29))
            (LocalVariables|Setbest_distance%28local%29 (LocalVariables|Getcurrent_distance%28local%29))
            (if (Variables|TimesUpgraded|GetIsLaiser)
              (Development|SetHiddeninGame (Variables|Default|GetNS_Laser) false false))
            (else
              (Development|SetHiddeninGame (Variables|Default|GetNS_Laser) true false)))))))
  ;[1 1 1] set the best target to the current target of the tower at the end of the loop
  (Variables|Private|SetTarget (LocalVariables|Getbest_target%28local%29)))

(fn UpdateTowerRotation
  (params (DeltaSeconds :type Float%20%28double-precision%29))
  ;[1 1 1] clamp the vertical angle to avoid clipping
  (bind _output_get (LocalVariables|SetNewRotator (Class|KismetMathLibrary|RInterptoConstant (Transformation|GetWorldRotation (Variables|Default|GetHead)) (Math|Rotator|FindLookatRotation (Transformation|GetWorldLocation (Variables|Default|GetHead)) (Transformation|GetActorLocation (Variables|Private|GetTarget))) DeltaSeconds (Variables|constant|GetInterp%20Speed))))
  ;[1 1 1] aplying the rotation
  (Transformation|SetWorldRotation (Variables|Default|GetHead) (Math|Rotator|MakeRotator (.roll _output_get) (Math|Float|ClampAngle (.pitch _output_get) -45.0 8e+01) (.yaw _output_get)) false false))

(fn UpdateFire
  (if (> (- (Utilities|Time|GetGameTimeinSeconds) (Variables|Private|GetTimeOfLastFire)) (Variables|Upgradeble|GetRateOfFire)) ; has cooldown?
    ;[1 1 1] Tower Facing Enemy?
    (if (> (Math|Vector|DotProduct (Math|Vector|GetUnitDirection(Vector) (Transformation|GetWorldLocation (Variables|Default|GetHead)) (Transformation|GetActorLocation (Variables|Private|GetTarget))) (Math|Vector|GetForwardVector (Variables|Default|GetHead))) 0.8)
      (Development|PrintString "Fire!!!!!")
      (if (Variables|TimesUpgraded|GetIsLaiser)
        (CallFunction|FireLaiser)
        (else
          (CallFunction|FireBullet))))))

(fn UpgradeFireRate
  (params (FR_UpgradeValue :type Float%20%28double-precision%29) (TimesUpgraded :type Integer))
  (if (Variables|TimesUpgraded|GetIsLaiser)
    (if (and (<= (Variables|Upgradeble|GetRateOfFire) (Variables|DefaultValues|GetDefaultFireRate)) (>= (Variables|Upgradeble|GetRateOfFire) 0.2))
      (Variables|Upgradeble|SetRateOfFire (- (Variables|Upgradeble|GetRateOfFire) (* FR_UpgradeValue TimesUpgraded)))
      (Variables|TimesUpgraded|SetFRTiems (+ (Variables|TimesUpgraded|GetFRTiems) 1))
      (Development|PrintString "FireRateIncreasedAsNeeded" true true "(R=0.666800,G=0.000000,B=1.000000,A=1.000000)"))))

(fn UpgradeRange
  (params (R_UpgradeValue :type Float%20%28double-precision%29) (TimesUpgraded :type Integer))
  (if (Variables|TimesUpgraded|GetIsLaiser)
    (if (and (>= (Variables|Upgradeble|Getsensing_range) (Variables|DefaultValues|GetDefaultSensingRange)) (<= (Variables|Upgradeble|Getsensing_range) 5e+03))
      (Variables|Upgradeble|Setsensing_range (+ (Variables|Upgradeble|Getsensing_range) (* R_UpgradeValue TimesUpgraded)))
      (Variables|TimesUpgraded|SetRTimes (+ (Variables|TimesUpgraded|GetRTimes) 1))
      (Development|PrintString "RangeUpgradedAzNeeded" true true "(R=0.985079,G=0.000000,B=1.000000,A=1.000000)"))))

(fn UpgradeBulletDamage
  (params (D_UpgradeValue :type Float%20%28double-precision%29) (TimesUpgraded :type Integer))
  (if (Variables|TimesUpgraded|GetIsLaiser)
    (if (and (>= (Variables|Upgradeble|GetDamage) (Variables|DefaultValues|GetDefaultDamage)) (< (Variables|Upgradeble|GetDamage) 3e+01))
      (Variables|Upgradeble|SetDamage (+ (Variables|Upgradeble|GetDamage) (* D_UpgradeValue TimesUpgraded)))
      (Variables|TimesUpgraded|SetDTimes (+ (Variables|TimesUpgraded|GetDTimes) 1)))))

(fn SetBaseAtts
  (CallFunction|SetDefaults)
  (CallFunction|BulletTower))