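; Checkpoint actor that feeds its position relative to the player into the minimap.
; After a tiny BeginPlay delay, it attaches its Helper component to the player pawn's root.
; Each tick it moves Helper back to the checkpoint's world location, so Helper's relative location becomes the checkpoint's offset in player space.
; That offset is flattened to 2D and passed to BP_FirstPersonCharacter's UpdateMiniMap, avoiding manual transform math.
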(event EventBeginPlay
  (bind _helper (Variables|Default|GetHelper))
  (Utilities|FlowControl|Delay 0.0001)
  (Transformation|AttachComponentToComponent (Variables|Default|GetHelper) (Variables|/Script/Engine.Actor|GetRootComponent (Game|Player|GetPlayerPawn 0)) "None" "KeepWorld" "KeepWorld" "KeepWorld" true)
  (Transformation|SetWorldLocation _helper (Transformation|GetActorLocation) false false)
  (bind _asbp_first_person_character (Utilities|Casting|CastToBP_FirstPersonCharacter (Game|Player|GetPlayerPawn 0)))
  (Default|UpdateMiniMap _asbp_first_person_character (Math|Conversions|ToVector2D(Vector) (Variables|/Script/Engine.SceneComponent|GetRelativeLocation _helper))))

(event EventTick
  (params (DeltaSeconds :type Float%20%28single-precision%29))
  (bind _helper (Variables|Default|GetHelper))
  (Transformation|SetWorldLocation _helper (Transformation|GetActorLocation) false false)
  (bind _asbp_first_person_character (Utilities|Casting|CastToBP_FirstPersonCharacter (Game|Player|GetPlayerPawn 0)))
  (Default|UpdateMiniMap _asbp_first_person_character (Math|Conversions|ToVector2D(Vector) (Variables|/Script/Engine.SceneComponent|GetRelativeLocation _helper))))

(fn ConstructionScript)