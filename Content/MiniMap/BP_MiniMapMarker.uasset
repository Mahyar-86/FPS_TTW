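; BP_MiniMapMarker is a marker actor that shows its icon on the player's minimap.
; BeginPlay creates a WBP_MiniMapIcon widget and attaches the Helper component to the player pawn's root.
; Each Tick moves Helper to the marker's world position and feeds its relative location to the widget as 2D, letting attachment convert coordinates into player space.
; The construction script applies the icon and screen size to a Billboard.
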(event EventBeginPlay
  (bind _helper (Variables|Default|GetHelper))
  (Utilities|FlowControl|Delay 0.0001)
  (bind _returnvalue (UserInterface|CreateWidget "/Game/MiniMap/WBP_MiniMapIcon.WBP_MiniMapIcon_C"))
  (bind _output_get (Variables|Default|SetMiniMapIconWidget _returnvalue))
  (Default|ChangeIcon _output_get (Variables|Default|GetMarkerIcon) (Variables|Default|GetMiniMapSize))
  (UserInterface|Viewport|AddtoViewport _output_get 0)
  (Transformation|AttachComponentToComponent (Variables|Default|GetHelper) (Variables|/Script/Engine.Actor|GetRootComponent (Game|Player|GetPlayerPawn 0)) "None" "KeepWorld" "KeepWorld" "KeepWorld" true)
  (Transformation|SetWorldLocation _helper (Transformation|GetActorLocation) false false)
  (bind _minimapiconwidget (Variables|Default|GetMiniMapIconWidget)
    (:then
      (Default|UpdateMiniMapIcon _minimapiconwidget (Math|Conversions|ToVector2D(Vector) (Variables|/Script/Engine.SceneComponent|GetRelativeLocation _helper))))
    (:else)))

(event EventTick
  (params (DeltaSeconds :type Float%20%28single-precision%29))
  (bind _helper (Variables|Default|GetHelper))
  (Transformation|SetWorldLocation _helper (Transformation|GetActorLocation) false false)
  (bind _minimapiconwidget (Variables|Default|GetMiniMapIconWidget)
    (:then
      (Default|UpdateMiniMapIcon _minimapiconwidget (Math|Conversions|ToVector2D(Vector) (Variables|/Script/Engine.SceneComponent|GetRelativeLocation _helper))))
    (:else)))

(fn ConstructionScript
  (bind _billboard (Variables|Default|GetBillboard))
  (Rendering|Components|Sprite|SetSprite _billboard (Variables|Default|GetMarkerIcon))
  (Variables|/Script/Engine.BillboardComponent|SetScreenSize _billboard (Variables|Default|GetScreen%20Size)))