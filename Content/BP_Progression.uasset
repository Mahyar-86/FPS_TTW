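; BP_Progression drives wave-based difficulty and unlocks, reacting to the game mode's Progress event.
; Each Progress updates spawn zones' enemy count, speed and sensing, plus fog density.
; Specific waves unlock dash, reveal traps, or open a widget offering two seeded-random modifiers: object heights, fog, more enemies, ghost mode or slow enemies.
; The chosen modifier is applied through the same setters, with manual flags overriding fog and sensing progression.
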(event Custom|Progress
  ;[0.05127 0.05127 0.05127] Set Progress Flow
  (Utilities|FlowControl|Sequence
    (:then_0
      (bind _asbp_first_person_game_mode (Utilities|Casting|CastToBP_FirstPersonGameMode (Game|GetGameMode)))
      (switch int (Variables|/Game/FirstPerson/Blueprints/BP_FirstPersonGameMode.BP_FirstPersonGameMode_C|GetWave _asbp_first_person_game_mode)
        (:0
          (CallFunction|ChooseProgress :!label _label))
        (:1
          (goto _label))
        (:3
          (goto _label))
        (:5
          (CallFunction|EnableDashAbility))
        (:7
          (goto _label))
        (:11
          (goto _label))
        (:13
          (CallFunction|EnableTraps))
        (:15
          (goto _label))
        (:19
          (goto _label))))
    (:then_1
      (CallFunction|ChangeEnemySpawner)
      (CallFunction|SetEnemyCount)
      (CallFunction|SetEnemySpeed 8e+02)
      (CallFunction|SetEnemySensing)
      (CallFunction|SetFog))))

(event Custom|EnableDashAbility
  ;[0.05127 0.05127 0.05127] Progress Functions
  ;;[0.05127 0.05127 0.05127] Enable Dash Ability
  (bind _returnvalue (Actor|GetActorOfClass "/Game/FirstPerson/Upgrade/Blueprints/BP_DashAbility.BP_DashAbility_C"))
  (Default|EnableDashAbility _returnvalue))

(event Custom|SetEnemySpeed
  (params (WalkSpeed :type Float%20%28single-precision%29))
  ;[0.05127 0.05127 0.05127] Progress Functions
  ;;[0.05127 0.05127 0.05127] Set Enemy Walk Speed
  (bind _outactors (Actor|GetAllActorsOfClass "/Game/BP_SpawnZone.BP_SpawnZone_C"))
  (for _array_element _outactors
    (Variables|/Game/BP_SpawnZone.BP_SpawnZone_C|SetWalkSpeed _array_element WalkSpeed)))

(event Custom|ChangeEnemySpawner
  ;[0.05127 0.05127 0.05127] Progress Functions
  ;;[0.05127 0.05127 0.05127] Enable Enemy Spawners
  (bind _outactors (Actor|GetAllActorsOfClass "/Game/BP_SpawnZone.BP_SpawnZone_C"))
  (for _array_element _outactors
    (bind _output_get (Variables|/Game/BP_SpawnZone.BP_SpawnZone_C|SetWichEnemySpawner _array_element 1))
    (Variables|Default|SetWichEnemySpawner _output_get)))

(event Custom|EnableTraps
  ;[0.05127 0.05127 0.05127] Progress Functions
  ;;[0.05127 0.05127 0.05127] Enable Traps
  (Utilities|FlowControl|Sequence
    (:then_0
      (bind _outactors (Actor|GetAllActorsOfClass "/Game/Trap/Spike/BP_SpikeTrap.BP_SpikeTrap_C"))
      (for _array_element _outactors
        (Rendering|SetActorHiddenInGame _array_element false)))
    (:then_1
      (bind _outactors_2 (Actor|GetAllActorsOfClass "/Game/Trap/Spike/BP_SpikeTrapKey.BP_SpikeTrapKey_C"))
      (for _array_element_2 _outactors_2
        (Rendering|SetActorHiddenInGame _array_element_2 false)
        (Variables|/Game/Trap/Spike/BP_SpikeTrapKey.BP_SpikeTrapKey_C|SetCanWork _array_element_2 true)))
    (:then_2
      (bind _asbp_first_person_game_mode (Utilities|Casting|CastToBP_FirstPersonGameMode (Game|GetGameMode)))
      (Default|PrintText _asbp_first_person_game_mode "Now You Can Enable Traps"))))

(event Custom|ChangeSunPlace
  ;[0.05127 0.05127 0.05127] Progress Functions
  ;;[0.05127 0.05127 0.05127] Random Sun
  (bind _asbp_first_person_game_mode (Utilities|Casting|CastToBP_FirstPersonGameMode (Game|GetGameMode)))
  (if (Variables|/Game/FirstPerson/Blueprints/BP_FirstPersonGameMode.BP_FirstPersonGameMode_C|GetDynamicLight _asbp_first_person_game_mode)
    (bind _returnvalue (Actor|GetActorOfClass "/Script/Engine.DirectionalLight"))
    (Transformation|SetMobility (Variables|/Script/Engine.Light|GetLightComponent _returnvalue) "Movable")
    (Transformation|SetActorRotation _returnvalue (Math|Rotator|MakeRotator 0.0 (Math|Random|RandomFloatinRange 1.8e+02 3.6e+02) (Math|Random|RandomFloatinRange 0.0 3.6e+02)))
    (Transformation|SetMobility (Variables|/Script/Engine.Light|GetLightComponent _returnvalue) "Static")))

(event Custom|SetChoosedProgress
  (bind _targetenemyspawner (Variables|Default|GetTargetEnemySpawner))
  ;[0.05127 0.05127 0.05127] Progress Functions
  ;;[0.05127 0.05127 0.05127] Choose Next Progress Changes by Player
  (switch Utilities|FlowControl|Switch|SwitchonE_ChooseProgress (Variables|Default|GetNextProgress)
    (:NewEnumerator0
      (CallFunction|SetRandomHeight))
    (:NewEnumerator1
      (Variables|Default|SetManualFog true)
      (CallFunction|SetFog))
    (:NewEnumerator2
      (for _array_element _targetenemyspawner
        (Variables|/Game/BP_SpawnZone.BP_SpawnZone_C|SetEnemySpawned _array_element (/ (+ (Variables|Default|GetEnemyCount) (Variables|Default|GetChangedEnemyCount)) (Utilities|Array|Length _targetenemyspawner)))))
    (:NewEnumerator6
      (Variables|Default|SetManualSensing true)
      (CallFunction|SetEnemySensing))
    (:NewEnumerator7
      (CallFunction|SetEnemySpeed 2e+02))))

(event Custom|SetRandomHeight
  ;[0.05127 0.05127 0.05127] Progress Functions
  ;;[0.05127 0.05127 0.05127] Set Random Height for Objects
  (bind _outactors (Actor|GetAllActorsOfClass "/Game/MapObjects/BP_Object.BP_Object_C"))
  (for _array_element _outactors
    (if (not (Variables|/Game/MapObjects/BP_Object.BP_Object_C|GetisNotMovable _array_element))
      (switch int (Math|Random|RandomInteger 10)
        (:0
          (Variables|Default|SetZChange -14602.0 :!label _label))
        (:1
          (goto _label))
        (:2
          (goto _label))
        (:3
          (goto _label))
        (:4
          (goto _label))
        (:5
          (Variables|Default|SetZChange -15202.0 :!label _label_2))
        (:6
          (goto _label_2))
        (:7
          (goto _label_2))
        (:8
          (Variables|Default|SetZChange -15502.0 :!label _label_3))
        (:9
          (goto _label_3)))
      (Transformation|SetActorLocation _array_element (Math|Vector|MakeVector (.x (Transformation|GetWorldLocation (Variables|/Game/MapObjects/BP_Object.BP_Object_C|GetDefaultSceneRoot _array_element))) (.y (Transformation|GetWorldLocation (Variables|/Game/MapObjects/BP_Object.BP_Object_C|GetDefaultSceneRoot _array_element))) (Variables|Default|GetZChange)) false false))))

(event Custom|SetFog
  ;[0.05127 0.05127 0.05127] Progress Functions
  ;;[0.05127 0.05127 0.05127] Set Fog Density
  (bind _returnvalue (Actor|GetActorOfClass "/Script/Engine.ExponentialHeightFog"))
  (if (Variables|Default|GetManualFog)
    (Class|ExponentialHeightFogComponent|SetFogDensity (Variables|/Script/Engine.ExponentialHeightFog|GetComponent _returnvalue) 0.04)
    (Variables|Default|SetManualFog false :!label _label)
    (elif (>= (Variables|/Script/Engine.ExponentialHeightFogComponent|GetFogDensity (Variables|/Script/Engine.ExponentialHeightFog|GetComponent _returnvalue)) (Variables|Default|GetMaxFog))
      (Class|ExponentialHeightFogComponent|SetFogDensity (Variables|/Script/Engine.ExponentialHeightFog|GetComponent _returnvalue) (+ (Variables|/Script/Engine.ExponentialHeightFogComponent|GetFogDensity (Variables|/Script/Engine.ExponentialHeightFog|GetComponent _returnvalue)) 0.0025))
      (goto _label))))

(event Custom|SetEnemySensing
  ;[0.05127 0.05127 0.05127] Progress Functions
  ;;[0.05127 0.05127 0.05127] Set Enemy Sensing Range
  (bind _outactors (Actor|GetAllActorsOfClass "/Game/BP_SpawnZone.BP_SpawnZone_C"))
  (for _array_element _outactors
    (if (Variables|Default|GetManualSensing)
      (Variables|/Game/BP_SpawnZone.BP_SpawnZone_C|SetSensingRange _array_element (Variables|Default|GetChangedEnemySensingRange))
      (Variables|Default|SetManualSensing false :!label _label)
      (elif (>= (Variables|Default|GetProgressSensingRange) 5e+02)
        (bind _output_get (Variables|Default|SetProgressSensingRange (- (Variables|Default|GetProgressSensingRange) 25.0)))
        (Variables|/Game/BP_SpawnZone.BP_SpawnZone_C|SetSensingRange _array_element _output_get)
        (goto _label)))))

(event Custom|SetEnemyCount
  (bind _targetenemyspawner (Variables|Default|GetTargetEnemySpawner))
  (bind _targetenemyspawner_2 (Variables|Default|GetTargetEnemySpawner))
  (bind _increasedenemycount (Variables|Default|GetIncreasedEnemyCount))
  ;[0.05127 0.05127 0.05127] Progress Functions
  ;;[0.05127 0.05127 0.05127] Set Enemy Count
  (Math|Integer|IncrementInt _increasedenemycount
    (:%20%20
      (Variables|Default|SetEnemyCount (+ (Variables|Default|GetEnemyCount) _increasedenemycount))
      (bind _outactors (Actor|GetAllActorsOfClass "/Game/BP_SpawnZone.BP_SpawnZone_C"))
      (for _array_element _outactors
        (if (== (Variables|Default|GetWichEnemySpawner) (Variables|/Game/BP_SpawnZone.BP_SpawnZone_C|GetSpawnerVersion _array_element))
          (Utilities|Array|Add _targetenemyspawner _array_element)
          (for _array_element_2 _targetenemyspawner_2
            (Variables|/Game/BP_SpawnZone.BP_SpawnZone_C|SetEnemySpawned _array_element_2 (/ (Variables|Default|GetEnemyCount) (Utilities|Array|Length _targetenemyspawner)))
            (Utilities|FlowControl|Delay 1.0)
            (Utilities|Array|Clear _targetenemyspawner_2)))))))

(event Custom|ChooseProgress
  (bind _chooseprogressstream (Variables|Default|GetChooseProgressStream))
  ;[0.05127 0.05127 0.05127] Progress Functions
  ;;[0.05127 0.05127 0.05127] Choose Next Progress Changes by Player
  (bind _returnvalue (UserInterface|CreateWidget "/Game/UI/widgets/WBP_ChooseProgress.WBP_ChooseProgress_C"))
  (UserInterface|Viewport|AddtoViewport _returnvalue 0)
  (EventDispatchers|BindEventtoNextProgressChoosed (delegate Custom|SetChoosedProgress))
  (Variables|Default|SetProgressOption1 (Utilities|Select :Index (Class|KismetMathLibrary|RandomIntegerfromStream _chooseprogressstream 5) :Option%200 "NewEnumerator0" :Option%201 "NewEnumerator1" :Option%202 "NewEnumerator2" :Option%203 "NewEnumerator6" :Option%204 "NewEnumerator7"))
  (Class|KismetMathLibrary|SeedRandomStream (Variables|Default|GetChooseProgressStream))
  (Variables|Default|SetProgressOption2 (Utilities|Select :Index (Class|KismetMathLibrary|RandomIntegerfromStream _chooseprogressstream 5) :Option%200 "NewEnumerator0" :Option%201 "NewEnumerator1" :Option%202 "NewEnumerator2" :Option%203 "NewEnumerator6" :Option%204 "NewEnumerator7")))

(event EventBeginPlay
  ;[0.05127 0.05127 0.05127] Call Make Progress
  (bind _asbp_first_person_game_mode (Utilities|Casting|CastToBP_FirstPersonGameMode (Game|GetGameMode)))
  (EventDispatchers|BindEventtoProgress _asbp_first_person_game_mode (delegate Custom|Progress)))

(fn ConstructionScript)