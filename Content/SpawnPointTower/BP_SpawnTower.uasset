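; Tower build spot where the player buys a shooter, bomb or ice tower outside attack waves.
; Box overlap enables input and shows a prompt; F opens the build menu, and leaving removes both.
; Number keys check game mode Currency, then spawn the tower with sound and destroy the marker meshes, or briefly show a credit warning.
; Tick polls FightTime to hide the spot during waves, and overlap ignores entry then.
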(event OnComponentEndOverlap(Box)
  (params (OverlappedComponent :type Primitive%20Component%20Object%20Reference) (OtherActor :type Actor%20Object%20Reference) (OtherComp :type Primitive%20Component%20Object%20Reference) (OtherBodyIndex :type Integer))
  (bind _tiwer_widget_1 (Variables|Default|Gettiwer%20widget%201))
  ;[1 1 1] Disable Spawning so player cannot spawn multiply towers in same place
  (Utilities|Casting|CastToBP_FirstPersonCharacter OtherActor)
  (Input|DisableInput (Game|GetPlayerController 0))
  (if (Variables|Default|Getwidget%20is%20in%20game%20view)
    (Widget|RemovefromParent (Variables|Default|Gettower%20widget))
    (Utilities|IsValid _tiwer_widget_1
      (:Is%20Valid
        (Widget|RemovefromParent _tiwer_widget_1))
      (:Is%20Not%20Valid
        _))
    (Variables|Default|Setis%20in%20tower false)
    (Variables|Default|Setwidget%20is%20in%20game%20view false)
    (Variables|Default|Setpressed%20f false)))

(event OnComponentBeginOverlap(Box)
  (params (OverlappedComponent :type Primitive%20Component%20Object%20Reference) (OtherActor :type Actor%20Object%20Reference) (OtherComp :type Primitive%20Component%20Object%20Reference) (OtherBodyIndex :type Integer) (bFromSweep :type Boolean) (SweepResult :type Hit%20Result%20Structure%20%28by%20ref%29))
  ;[1 1 1] Enabling Input so we can assign keys for spawning
  (if (not (Variables|/Game/FirstPerson/Blueprints/BP_FirstPersonGameMode.BP_FirstPersonGameMode_C|GetFightTime? (stale EventTick _asbp_first_person_game_mode)))
    (bind _asbp_first_person_character (Utilities|Casting|CastToBP_FirstPersonCharacter OtherActor))
    (Input|EnableInput (Game|GetPlayerController 0))
    (bind _returnvalue (UserInterface|CreateWidget "/Game/UI/create_tower.create_tower_C"))
    (bind _output_get (Variables|Default|Settower%20widget _returnvalue))
    (UserInterface|Viewport|AddtoViewport _output_get 0)
    (Variables|Default|Setwidget%20is%20in%20game%20view true)
    (Variables|Default|Setis%20in%20tower true)))

(event EventTick
  (params (DeltaSeconds :type Float%20%28single-precision%29))
  ;[1 1 1] Disable Spawner in Attack Wave
  (bind _asbp_first_person_game_mode (Utilities|Casting|CastToBP_FirstPersonGameMode (Game|GetGameMode)))
  (if (Variables|/Game/FirstPerson/Blueprints/BP_FirstPersonGameMode.BP_FirstPersonGameMode_C|GetFightTime? _asbp_first_person_game_mode)
    (Rendering|SetActorHiddenInGame true)
    (else
      (Rendering|SetActorHiddenInGame false))))

(event Input|KeyboardEvents|F
  (params (Key :type Key%20Structure :default "None"))
  ;[1 1 1] Stuff for opening construction menu
  (:Pressed
    (if (Variables|Default|Getis%20in%20tower)
      (bind _returnvalue (UserInterface|CreateWidget "/Game/UI/create_tower1.create_tower1_C"))
      (bind _output_get (Variables|Default|Settiwer%20widget%201 _returnvalue))
      (UserInterface|Viewport|AddtoViewport _output_get 0)
      (Variables|Default|Setpressed%20f true))))

(event Input|KeyboardEvents|1
  (params (Key :type Key%20Structure :default "None"))
  ;[0.156 0.6619 1] Spawning and checking credits
  (:Pressed
    (if (Variables|Default|Getpressed%20f)
      (bind _asbp_first_person_game_mode (Utilities|Casting|CastToBP_FirstPersonGameMode (Game|GetGameMode)))
      (if (>= (Variables|/Game/FirstPerson/Blueprints/BP_FirstPersonGameMode.BP_FirstPersonGameMode_C|GetCurrency _asbp_first_person_game_mode) 50)
        (Variables|/Game/FirstPerson/Blueprints/BP_FirstPersonGameMode.BP_FirstPersonGameMode_C|SetCurrency _asbp_first_person_game_mode (- (Variables|/Game/FirstPerson/Blueprints/BP_FirstPersonGameMode.BP_FirstPersonGameMode_C|GetCurrency _asbp_first_person_game_mode) 50))
        (Game|SpawnActorfromClass "/Game/Tower/BP_ShooterTower.BP_ShooterTower_C" (Transformation|GetWorldTransform (Variables|Default|GetBox self)) "Undefined" "MultiplyWithRoot" (stale OnComponentBeginOverlap(Box) _asbp_first_person_character) 0)
        (Audio|SpawnSoundAttached "/Game/Sounds/Towers/LaserTower.LaserTower" (Variables|Default|GetBox) "None" "0, 0, 0" "0, 0, 0" "KeepRelativeOffset" false 1.0 1.0 0.0 "/Game/Sounds/SA_SoundAttenuation.SA_SoundAttenuation" 0)
        (Components|DestroyComponent (Variables|Default|GetCone))
        (else
          ;[1 1 1] Have no currency Warn
          (bind _asbp_first_person_game_mode_2 (Utilities|Casting|CastToBP_FirstPersonGameMode (Game|GetGameMode)))
          (Variables|/Game/FirstPerson/Blueprints/BP_FirstPersonGameMode.BP_FirstPersonGameMode_C|SetUpgradeText _asbp_first_person_game_mode_2 "Not enough Credits")
          (bind _returnvalue (UserInterface|CreateWidget "/Game/UI/widgets/W_Upgrades.W_Upgrades_C"))
          (UserInterface|Viewport|AddtoViewport _returnvalue 0)
          (Utilities|FlowControl|Delay 5.0)
          (Widget|RemovefromParent _returnvalue))))))

(event Input|KeyboardEvents|2
  (params (Key :type Key%20Structure :default "None"))
  ;[0.156 0.6619 1] Spawning and checking credits
  (:Pressed
    (if (Variables|Default|Getpressed%20f)
      (bind _asbp_first_person_game_mode (Utilities|Casting|CastToBP_FirstPersonGameMode (Game|GetGameMode)))
      (if (>= (Variables|/Game/FirstPerson/Blueprints/BP_FirstPersonGameMode.BP_FirstPersonGameMode_C|GetCurrency _asbp_first_person_game_mode) 100)
        (Variables|/Game/FirstPerson/Blueprints/BP_FirstPersonGameMode.BP_FirstPersonGameMode_C|SetCurrency _asbp_first_person_game_mode (- (Variables|/Game/FirstPerson/Blueprints/BP_FirstPersonGameMode.BP_FirstPersonGameMode_C|GetCurrency _asbp_first_person_game_mode) 100))
        (Game|SpawnActorfromClass "/Game/BombTower/BP_BTower.BP_BTower_C" (Transformation|GetWorldTransform (Variables|Default|GetBox self)) "Undefined" "MultiplyWithRoot" (stale OnComponentBeginOverlap(Box) _asbp_first_person_character) 0)
        (Audio|SpawnSoundAttached "/Game/Sounds/Towers/BombTower.BombTower" (Variables|Default|GetBox) "None" "0, 0, 0" "0, 0, 0" "KeepRelativeOffset" false 1.0 1.0 0.0 "/Game/Sounds/SA_SoundAttenuation.SA_SoundAttenuation" 0)
        (Components|DestroyComponent (Variables|Default|GetCone))
        (else
          ;[1 1 1] Have no currency Warn
          (bind _asbp_first_person_game_mode_2 (Utilities|Casting|CastToBP_FirstPersonGameMode (Game|GetGameMode)))
          (Variables|/Game/FirstPerson/Blueprints/BP_FirstPersonGameMode.BP_FirstPersonGameMode_C|SetUpgradeText _asbp_first_person_game_mode_2 "Not enough Credits")
          (bind _returnvalue (UserInterface|CreateWidget "/Game/UI/widgets/W_Upgrades.W_Upgrades_C"))
          (UserInterface|Viewport|AddtoViewport _returnvalue 0)
          (Utilities|FlowControl|Delay 5.0)
          (Widget|RemovefromParent _returnvalue))))))

(event Input|KeyboardEvents|3
  (params (Key :type Key%20Structure :default "None"))
  ;[0.156 0.6619 1] Spawning and checking credits
  (:Pressed
    (if (Variables|Default|Getpressed%20f)
      (bind _asbp_first_person_game_mode (Utilities|Casting|CastToBP_FirstPersonGameMode (Game|GetGameMode)))
      (if (>= (Variables|/Game/FirstPerson/Blueprints/BP_FirstPersonGameMode.BP_FirstPersonGameMode_C|GetCurrency _asbp_first_person_game_mode) 50)
        (Variables|/Game/FirstPerson/Blueprints/BP_FirstPersonGameMode.BP_FirstPersonGameMode_C|SetCurrency _asbp_first_person_game_mode (- (Variables|/Game/FirstPerson/Blueprints/BP_FirstPersonGameMode.BP_FirstPersonGameMode_C|GetCurrency _asbp_first_person_game_mode) 50))
        (Game|SpawnActorfromClass "/Game/IceTower/BP_IceTower.BP_IceTower_C" (Transformation|GetWorldTransform (Variables|Default|GetBox self)) "AlwaysSpawn" "MultiplyWithRoot" (stale OnComponentBeginOverlap(Box) _asbp_first_person_character) 0)
        (Audio|SpawnSoundAttached "/Game/Sounds/Towers/Ice.Ice" (Variables|Default|GetBox) "None" "0, 0, 0" "0, 0, 0" "KeepRelativeOffset" false 1.0 1.0 0.0 "/Game/Sounds/SA_SoundAttenuation.SA_SoundAttenuation" 0)
        (Components|DestroyComponent (Variables|Default|GetCone))
        (else
          ;[1 1 1] Have no currency Warn
          (bind _asbp_first_person_game_mode_2 (Utilities|Casting|CastToBP_FirstPersonGameMode (Game|GetGameMode)))
          (Variables|/Game/FirstPerson/Blueprints/BP_FirstPersonGameMode.BP_FirstPersonGameMode_C|SetUpgradeText _asbp_first_person_game_mode_2 "Not enough Credits")
          (bind _returnvalue (UserInterface|CreateWidget "/Game/UI/widgets/W_Upgrades.W_Upgrades_C"))
          (UserInterface|Viewport|AddtoViewport _returnvalue 0)
          (Utilities|FlowControl|Delay 5.0)
          (Widget|RemovefromParent _returnvalue))))))

(fn ConstructionScript)

(fn NewFunction)

(fn NewFunction0)