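; BP_IceTower is a tower actor that slows nearby BP_Zombie pawns.
; Every Tick it runs a sphere overlap around its root and lowers each zombie's CharacterMovement max walk speed.
; A one-second Delay inside the loop precedes the speed reset, so all iterations share one latent timer and the reset does not run per zombie.
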(event EventBeginPlay)

(event Collision|EventActorBeginOverlap
  (params (OtherActor :type Actor%20Object%20Reference)))

(event EventTick
  (params (DeltaSeconds :type Float%20%28single-precision%29))
  (bind _outactors (Collision|SphereOverlapActors (Transformation|GetWorldLocation (Variables|Default|GetDefaultSceneRoot)) 1e+03 (Utilities|Array|MakeArray "ObjectTypeQuery3") 0 (Utilities|Array|MakeArray self)))
  (for _array_element _outactors
    (bind _asbp_zombie (Utilities|Casting|CastToBP_Zombie _array_element))
    (Utilities|IsValid (Variables|/Script/Engine.Character|GetCharacterMovement _asbp_zombie)
      (:Is%20Valid
        (Variables|/Script/Engine.CharacterMovementComponent|SetMaxWalkSpeed (Variables|/Script/Engine.Character|GetCharacterMovement _asbp_zombie) 1e+02)
        (Utilities|FlowControl|Delay 1.0)
        (Utilities|IsValid (Variables|/Script/Engine.Character|GetCharacterMovement _asbp_zombie)
          (:Is%20Valid
            (Variables|/Script/Engine.CharacterMovementComponent|SetMaxWalkSpeed (Variables|/Script/Engine.Character|GetCharacterMovement _asbp_zombie) 3.6e+02)))))))

(fn ConstructionScript)