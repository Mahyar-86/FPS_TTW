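; BP_BombTower is a turret that reacts when a tagged actor enters its Sphere and fires a BP_Bullet.
; The overlap prints a debug string, checks for the "None" tag, then takes one interpolated look-at step, pitch-clamped on Tower and yaw-only on the actor.
; The look-at start and target both read the tower's own location, not the overlapping actor's.
; A short retriggerable delay then spawns the bullet at BomberHead's transform.
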(event OnComponentBeginOverlap(Sphere)
  (params (OverlappedComponent :type Primitive%20Component%20Object%20Reference) (OtherActor :type Actor%20Object%20Reference) (OtherComp :type Primitive%20Component%20Object%20Reference) (OtherBodyIndex :type Integer) (bFromSweep :type Boolean) (SweepResult :type Hit%20Result%20Structure%20%28by%20ref%29))
  (bind _returnvalue (Transformation|GetActorLocation))
  (bind _returnvalue_2 (Transformation|GetActorRotation))
  (bind _returnvalue_3 (Utilities|Time|GetWorldDeltaSeconds))
  (bind _returnvalue_4 (Transformation|GetActorLocation))
  (bind _returnvalue_5 (* 2e+01 5.0))
  (bind _returnvalue_6 (Math|Rotator|FindLookatRotation _returnvalue _returnvalue_4))
  (bind _returnvalue_7 (Math|Interpolation|RInterpTo _returnvalue_2 _returnvalue_6 _returnvalue_3 _returnvalue_5))
  (Development|PrintString "Hello" true true "(R=0.000000,G=0.660000,B=1.000000,A=1.000000)" 5.0)
  (if (Actor|ActorHasTag OtherActor "None")
    (Utilities|FlowControl|Sequence
      (:then_0
        (Transformation|SetWorldRotation (Variables|Default|Get%20Tower) (Math|Rotator|MakeRotator 0.0 (Math|Float|Clamp(Float) (.pitch _returnvalue_7) -2e+01 2e+01) (.yaw _returnvalue_7)) false false)
        (Transformation|SetActorRotation (Math|Rotator|MakeRotator 0.0 0.0 (.yaw _returnvalue_7))))
      (:then_1
        (Utilities|FlowControl|RetriggerableDelay 0.5)
        (Game|SpawnActorfromClass "/Game/Tower/BP_Bullet.BP_Bullet_C" (Transformation|GetWorldTransform (Variables|Default|GetBomberHead)) "Undefined" "MultiplyWithRoot" 0 0)))))

(fn ConstructionScript)