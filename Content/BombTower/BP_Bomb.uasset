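; BP_Bomb is the bomb actor of the bomb tower, damaging BP_Zombie1 enemies and exploding on contact.
; Zombies overlapping its Sphere take point damage, with the result printed for debugging.
; A zombie overlapping the Bomb component spawns an explosion emitter and destroys the actor.
; An uncalled RadialDamage function only returns a sphere-overlap result filtered on ABP_Zombie, applying no damage.
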(event OnComponentBeginOverlap(Sphere)
  (params (OverlappedComponent :type Primitive%20Component%20Object%20Reference) (OtherActor :type Actor%20Object%20Reference) (OtherComp :type Primitive%20Component%20Object%20Reference) (OtherBodyIndex :type Integer) (bFromSweep :type Boolean) (SweepResult :type Hit%20Result%20Structure%20%28by%20ref%29))
  (bind _asbp_zombie (Utilities|Casting|CastToBP_Zombie1 OtherActor))
  (bind _returnvalue (Game|Damage|ApplyPointDamage _asbp_zombie 1e+01 (Math|Vector|GetForwardVector (Variables|Default|Get%20bomb)) SweepResult))
  (Development|PrintString (Utilities|String|ToString(Float) _returnvalue) true true "(R=1.000000,G=0.194100,B=0.000000,A=1.000000)"))

(event OnComponentBeginOverlap(bomb)
  (params (OverlappedComponent :type Primitive%20Component%20Object%20Reference) (OtherActor :type Actor%20Object%20Reference) (OtherComp :type Primitive%20Component%20Object%20Reference) (OtherBodyIndex :type Integer) (bFromSweep :type Boolean) (SweepResult :type Hit%20Result%20Structure%20%28by%20ref%29))
  (Utilities|Casting|CastToBP_Zombie1 OtherActor)
  (Effects|SpawnEmitteratLocation "/Game/Realistic_Starter_VFX_Pack_Vol2/Particles/Explosion/P_Explosion_Big_A.P_Explosion_Big_A" (Transformation|GetActorLocation) "0, 0, 0" "0.500000,0.500000,0.500000")
  (Actor|DestroyActor))

(fn ConstructionScript)

(fn RadialDamage
  (bind _outactors (Collision|SphereOverlapActors (Transformation|GetActorLocation) 5e+02 (Utilities|Array|MakeArray "ObjectTypeQuery3") "/Game/Zombie/Animations/ABP_Zombie.ABP_Zombie_C"))
  (for _array_element _outactors
    (return _array_element))
  (return _array_element))