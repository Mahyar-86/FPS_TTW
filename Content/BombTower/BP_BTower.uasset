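; Bomb tower that automatically targets nearby pawns, apparently zombies, and launches bombs at them.
; Each tick it sphere-overlaps its sensing range, skipping the player, and picks the closest pawn with line of sight.
; The head turns toward the target at constant speed with clamped pitch.
; Once the cooldown passes and a dot-product check confirms facing, it spawns BP_Bomb at the head with an explosion sound.
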(event Custom|Fire
  (bind _head (Variables|Default|GetHead))
  (bind _returnvalue (Transformation|GetWorldTransform _head))
  (Variables|Private|SetTimeOfLastFire (Utilities|Time|GetGameTimeinSeconds))
  (Utilities|FlowControl|Sequence
    (:then_0
      (goto _label Reset))
    (:then_1
      (Utilities|FlowControl|DoN 10 :!label _label
        (:Exit
          (Game|SpawnActorfromClass "/Game/BombTower/BP_Bomb.BP_Bomb_C" (Math|Transform|MakeTransform (+ (.location _returnvalue) "5.000000,0.000000,0.000000") (.rotation _returnvalue) (.scale _returnvalue)) "Undefined" "MultiplyWithRoot" 0 0)
          (Audio|SpawnSoundAttached "/Game/Sounds/Explosion01.Explosion01" (Variables|Default|GetHead) "None" "0, 0, 0" "0, 0, 0" "KeepRelativeOffset" false 1.0 1.0 0.0 "/Game/Sounds/SA_SoundAttenuation.SA_SoundAttenuation" 0))))))

(event EventTick
  (params (DeltaSeconds :type Float%20%28single-precision%29))
  (Private|FindBestTarget)
  (Variables|Private|GetTarget
    (:then
      (Private|UpdateTowerRotation DeltaSeconds)
      (Private|UpdateFire))
    (:else)))

(fn ConstructionScript)

(fn FindBestTarget
  ;[1 1 1] set the best distance var to the max
  (LocalVariables|Setbest_distance%28local%29 (+ (Variables|constant|Getsensing_range) 1.0))
  ;[1 1 1] detect zombies entering the sence zone
  (bind _outactors (Collision|SphereOverlapActors (Transformation|GetActorLocation) (Variables|constant|Getsensing_range) (Utilities|Array|MakeArray "ObjectTypeQuery3") 0 (Utilities|Array|MakeArray (Variables|Default|GetPlayer))))
  ;[1 1 1] looping through the array to find the closest target to the tower
  (for _array_element _outactors
    (bind _output_get (LocalVariables|Setcurrent_target%28local%29 _array_element))
    (Utilities|Casting|CastToBP_FirstPersonCharacter _output_get
      (:CastFailed
        (bind _output_get_2 (LocalVariables|Setcurrent_distance%28local%29 (Transformation|GetDistanceTo _output_get self)))
        (if (or (< _output_get_2 (LocalVariables|Getbest_distance%28local%29)) (not (Utilities|IsValid (LocalVariables|Getbest_target%28local%29)))) ; is this is the closest so far?
          (bind _result (CallFunction|HasLineOfSight (Transformation|GetWorldLocation (Variables|Default|GetHead)) (Transformation|GetActorLocation (LocalVariables|Getcurrent_target%28local%29)) (Utilities|Array|MakeArray self (LocalVariables|Getcurrent_target%28local%29) 0)))
          (if _result
            (LocalVariables|Setbest_target%28local%29 (LocalVariables|Getcurrent_target%28local%29))
            (LocalVariables|Setbest_distance%28local%29 (LocalVariables|Getcurrent_distance%28local%29)))))))
  ;[1 1 1] set the best target to the current target of the tower at the end of the loop
  (Variables|Private|SetTarget (LocalVariables|Getbest_target%28local%29)))

(fn UpdateTowerRotation
  (params (DeltaSeconds :type Float%20%28double-precision%29))
  ;[1 1 1] clamp the vertical angle to avoid clipping
  (bind _output_get (LocalVariables|SetNewRotator (Class|KismetMathLibrary|RInterptoConstant (Transformation|GetWorldRotation (Variables|Default|GetHead)) (Math|Rotator|FindLookatRotation (Transformation|GetWorldLocation (Variables|Default|GetHead)) (Transformation|GetActorLocation (Variables|Private|GetTarget))) DeltaSeconds (Variables|constant|GetInterp%20Speed))))
  ;[1 1 1] aplying the rotation
  (Transformation|SetWorldRotation (Variables|Default|GetHead) (Math|Rotator|MakeRotator (.roll _output_get) (Math|Float|ClampAngle (.pitch _output_get) -45.0 8e+01) (.yaw _output_get)) false false))

(fn UpdateFire
  (if (> (- (Utilities|Time|GetGameTimeinSeconds) (Variables|Private|GetTimeOfLastFire)) (Variables|constant|GetRateOfFire)) ; has cooldown?
    ;[1 1 1] Tower Facing Enemy?
    (if (> (Math|Vector|DotProduct (Math|Vector|GetUnitDirection(Vector) (Transformation|GetWorldLocation (Variables|Default|GetHead)) (Transformation|GetActorLocation (Variables|Private|GetTarget))) (Math|Vector|GetForwardVector (Variables|Default|GetHead))) 0.8)
      (Development|PrintString "Fire!!!!!")
      (CallFunction|Fire))))