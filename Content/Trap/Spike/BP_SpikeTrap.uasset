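; BP_SpikeTrap is a trap that raises spikes and hurts the player and zombies, active only while the game mode's SpikeTrap flag is set.
; A player entering the Box loses Health directly and triggers the spike rise; ending overlap lowers it after a delay.
; Tick sphere-scans for Zombie-tagged pawns, then after a short Delay reuses the rise and calls ApplyDamage.
; The game mode reference Tick uses is only cached on Box begin overlap.
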(event OnComponentBeginOverlap(Box)
  (params (OverlappedComponent :type Primitive%20Component%20Object%20Reference) (OtherActor :type Actor%20Object%20Reference) (OtherComp :type Primitive%20Component%20Object%20Reference) (OtherBodyIndex :type Integer) (bFromSweep :type Boolean) (SweepResult :type Hit%20Result%20Structure%20%28by%20ref%29))
  (bind _asbp_first_person_game_mode (Utilities|Casting|CastToBP_FirstPersonGameMode (Game|GetGameMode)))
  (if (Variables|/Game/FirstPerson/Blueprints/BP_FirstPersonGameMode.BP_FirstPersonGameMode_C|GetSpikeTrap _asbp_first_person_game_mode)
    (if (Actor|ActorHasTag OtherActor "Player")
      (bind _asbp_first_person_character (Utilities|Casting|CastToBP_FirstPersonCharacter (Game|Player|GetPlayerPawn 0)))
      (Variables|/Game/FirstPerson/Blueprints/BP_FirstPersonCharacter.BP_FirstPersonCharacter_C|SetHealth _asbp_first_person_character (- (Variables|/Game/FirstPerson/Blueprints/BP_FirstPersonCharacter.BP_FirstPersonCharacter_C|GetHealth _asbp_first_person_character) (Variables|Default|GetPlayerDamage)))
      (Components|MoveComponentTo (Variables|Default|GetSpikeTrap_Cube_001) "0, 0, 0" "0, 0, 0" false false 0.5 false))))

(event OnComponentEndOverlap(Box)
  (params (OverlappedComponent :type Primitive%20Component%20Object%20Reference) (OtherActor :type Actor%20Object%20Reference) (OtherComp :type Primitive%20Component%20Object%20Reference) (OtherBodyIndex :type Integer))
  (if (Variables|/Game/FirstPerson/Blueprints/BP_FirstPersonGameMode.BP_FirstPersonGameMode_C|GetSpikeTrap (stale OnComponentBeginOverlap(Box) _asbp_first_person_game_mode))
    (Utilities|FlowControl|Delay 1.0)
    (Components|MoveComponentTo (Variables|Default|GetSpikeTrap_Cube_001) "0.000000,0.000000,-100.000000" "0, 0, 0" false false 0.5 false)))

(event EventTick
  (params (DeltaSeconds :type Float%20%28single-precision%29))
  (if (Variables|/Game/FirstPerson/Blueprints/BP_FirstPersonGameMode.BP_FirstPersonGameMode_C|GetSpikeTrap (stale OnComponentBeginOverlap(Box) _asbp_first_person_game_mode))
    (bind _outactors (Collision|SphereOverlapActors (Transformation|GetWorldLocation (Variables|Default|GetDefaultSceneRoot)) 2e+02 (Utilities|Array|MakeArray "ObjectTypeQuery3") 0))
    (for _array_element _outactors
      (if (Actor|ActorHasTag _array_element "Zombie")
        (Utilities|FlowControl|Delay 0.2)
        (Utilities|FlowControl|Sequence
          (:then_0
            (Components|MoveComponentTo (Variables|Default|GetSpikeTrap_Cube_001) "0, 0, 0" "0, 0, 0" false false 0.5 false))
          (:then_1
            (bind _asbp_zombie (Utilities|Casting|CastToBP_Zombie _array_element))
            (Utilities|IsValid _asbp_zombie
              (:Is%20Valid
                (Game|Damage|ApplyDamage _asbp_zombie (Variables|Default|GetEnemy%20Damage) 0 0)))))))))

(fn ConstructionScript)