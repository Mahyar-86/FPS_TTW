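; BP_Base is the base that zombies attack, with game over when it is destroyed.
; Each tick it copies HitPoints to the first-person game mode, then sphere-scans nearby pawns and calls ApplyDamage on itself for each BP_Zombie found.
; AnyDamage subtracts a fixed amount and prints the remaining health.
; A damage event at zero health destroys the base, shows the W_Dead widget and cursor, and pauses the game.
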(event EventTick
  (params (DeltaSeconds :type Float%20%28single-precision%29))
  ;[1 1 1] Share Health With Game Mode
  (bind _asbp_first_person_game_mode (Utilities|Casting|CastToBP_FirstPersonGameMode (Game|GetGameMode)))
  (Variables|/Game/FirstPerson/Blueprints/BP_FirstPersonGameMode.BP_FirstPersonGameMode_C|SetBaseHealth _asbp_first_person_game_mode (Variables|Private|GetHitPoints))
  ;[1 1 1] Scan for enemies to take damage
  (bind _outactors (Collision|SphereOverlapActors (Transformation|GetActorLocation) 5e+02 (Utilities|Array|MakeArray "ObjectTypeQuery3") 0))
  (for _array_element _outactors
    (Utilities|Casting|CastToBP_Zombie _array_element)
    (Game|Damage|ApplyDamage self 0.0 0 0)))

(event Game|Damage|EventAnyDamage
  (params (Damage :type Float%20%28single-precision%29) (DamageType :type Damage%20Type%20Object%20Reference) (InstigatedBy :type Controller%20Object%20Reference) (DamageCauser :type Actor%20Object%20Reference))
  ;[1 1 1] On take damage
  (if (> (Variables|Private|GetHitPoints) 0.0)
    (bind _output_get (Variables|Private|SetHitPoints (- (Variables|Private|GetHitPoints) 1e+01)))
    (Development|PrintString (Utilities|String|ToString(Float) _output_get) true true "(R=1.000000,G=0.000000,B=0.049470,A=1.000000)" 5.0)
    (else
      (Actor|DestroyActor)
      (bind _returnvalue (UserInterface|CreateWidget "/Game/UI/widgets/W_Dead.W_Dead_C" (Game|GetPlayerController 0)))
      (UserInterface|Viewport|AddtoViewport _returnvalue 0)
      (Variables|/Script/Engine.PlayerController|SetbShowMouseCursor (Game|GetPlayerController 0) true)
      (Game|SetGamePaused true))))

(fn ConstructionScript)