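; Zombie spawn point actor that drives wave timing and spawning through BP_FirstPersonGameMode.
; On BeginPlay it passes its wait time to the game mode and binds SpawnEnemy to the RespawnEnemy event.
; SpawnEnemy delays around toggling Fight, spawns zombies and increments Wave only if SpawnerVersion matches WichEnemySpawner, then sets DeleteHUD after a delay.
; Tick copies Fight and DeleteHUD to the game mode every frame.
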(event Custom|SpawnEnemy
  (bind _spawnerversion (Variables|Default|GetSpawnerVersion))
  (bind _wichenemyspawner (Variables|Default|GetWichEnemySpawner))
  (bind _returnvalue (== _spawnerversion _wichenemyspawner))
  (Utilities|FlowControl|Delay (Variables|Default|GetWave%20Transition%20Time))
  (Variables|Default|SetFight? false)
  (Utilities|FlowControl|Delay (Variables|Default|GetTimer))
  (Variables|Default|SetFight? true)
  (Utilities|FlowControl|Sequence
    (:then_0
      (for _index (range 0 (- (Variables|Default|GetEnemySpawned) 1))
        (if _returnvalue
          (Game|SpawnActorfromClass "/Game/Zombie/BP_Zombie.BP_Zombie_C" (Transformation|GetActorTransform) "AlwaysSpawn" "MultiplyWithRoot" 0 0)))
      (if _returnvalue
        (bind _asbp_first_person_game_mode (Utilities|Casting|CastToBP_FirstPersonGameMode (Game|GetGameMode)))
        (Math|Integer|IncrementInt (Variables|/Game/FirstPerson/Blueprints/BP_FirstPersonGameMode.BP_FirstPersonGameMode_C|GetWave _asbp_first_person_game_mode))))
    (:then_1
      (Utilities|FlowControl|Delay 5.0)
      (Variables|Default|SetDeleteHUD true))))

(event EventTick
  (params (DeltaSeconds :type Float%20%28single-precision%29))
  (bind _asbp_first_person_game_mode (Utilities|Casting|CastToBP_FirstPersonGameMode (Game|GetGameMode)))
  (Variables|/Game/FirstPerson/Blueprints/BP_FirstPersonGameMode.BP_FirstPersonGameMode_C|SetFightTime? _asbp_first_person_game_mode (Variables|Default|GetFight?))
  (Variables|/Game/FirstPerson/Blueprints/BP_FirstPersonGameMode.BP_FirstPersonGameMode_C|SetDeleteHUD? _asbp_first_person_game_mode (Variables|Default|GetDeleteHUD)))

(event EventBeginPlay
  (bind _asbp_first_person_game_mode (Utilities|Casting|CastToBP_FirstPersonGameMode (Game|GetGameMode)))
  (Variables|/Game/FirstPerson/Blueprints/BP_FirstPersonGameMode.BP_FirstPersonGameMode_C|SetWaitTime _asbp_first_person_game_mode (Variables|Default|GetTimer))
  (EventDispatchers|BindEventtoRespawnEnemy _asbp_first_person_game_mode (delegate Custom|SpawnEnemy)))

(fn ConstructionScript)